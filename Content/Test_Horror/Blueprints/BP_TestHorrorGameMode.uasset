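; BP_TestHorrorGameMode is the game mode for the Test_Horror game and owns the player's on-screen GUI.
; On BeginPlay it creates a WB_GUI widget, stores it, adds it to the viewport and starts its fade-in.
; Its ShowInteract, SetQuest and FinishQuest events forward interaction prompt and quest updates straight to that widget.
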(event `self.ReceiveBeginPlay`
  (bind _returnvalue (`|CreateWidget` "/Game/Test_Horror/UI/WB_GUI.WB_GUI_C"))
  (bind _output_get (set `self.GUI` _returnvalue))
  (`UserWidget.AddToViewport` _output_get 0)
  (`/Game/Test_Horror/UI/WB_GUI.FadeInEvent` (`self.GUI`)))

(event `Show Interact`
  (params (Show :type Boolean))
  (`/Game/Test_Horror/UI/WB_GUI.Show Interact` (`self.GUI`) Show))

(event `Set Quest`
  (params (Task :type Text))
  (`/Game/Test_Horror/UI/WB_GUI.Set Quest` (`self.GUI`) Task))

(event `Finish Quest`
  (`/Game/Test_Horror/UI/WB_GUI.Finish Quest` (`self.GUI`)))

(fn `UserConstructionScript`)