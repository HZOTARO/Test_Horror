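; BP_TestHorrorCharacter is a player character Blueprint for the horror test that tunes look and movement on top of its parent class.
; BeginPlay limits the player camera manager's vertical view pitch.
; The Aim and Move overrides scale their inputs by CameraSpeed and WalkSpeed, treated as percentages, before passing them to the parent implementations.
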(event `self.ReceiveBeginPlay`
  (bind _returnvalue (`GameplayStatics.GetPlayerCameraManager` 0))
  (set `PlayerCameraManager.ViewPitchMin` -55.0 _returnvalue)
  (set `PlayerCameraManager.ViewPitchMax` 70.0 _returnvalue))

(fn `Aim`
  (params (Yaw :type "Float (single-precision)") (Pitch :type "Float (double-precision)"))
  (bind _returnvalue (/ (`self.Camera Speed`) 100.0))
  (`parent.Aim` (* Yaw _returnvalue) (* Pitch _returnvalue)))

(fn `Move`
  (params (`Left / Right` :type "Float (double-precision)") (`Forward / Backward` :type "Float (double-precision)"))
  (bind _returnvalue (/ (`self.Walk Speed`) 100.0))
  (`parent.Move` (* `Left / Right` _returnvalue) (* `Forward / Backward` _returnvalue)))

(fn `UserConstructionScript`
  (`parent.UserConstructionScript`))