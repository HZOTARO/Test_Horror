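; Event manager that steps through an ordered chain of triggers in the horror test game, with only one activated at a time.
; BeginPlay activates the entry with ID 0 in the Triggers map.
; TriggerCurrentEvent calls OnEventComplete for IDs 0 to 2, all wired to the same call with no event-specific logic.
; It then destroys the current trigger if valid, increments CurrentId and activates the next valid one.
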(event `self.ReceiveBeginPlay`
  (set `/Game/Test_Horror/Blueprints/Item/BP_Collectible.Active` true (`BlueprintMapLibrary.Map_Find` (`self.Triggers`))))

(event `Trigger Current Event`
  (bind _value (`BlueprintMapLibrary.Map_Find` (`self.Triggers`) (`self.Current Id`)))
  (`|ExecutionSequence`
    (:`then_0`
      (switch `int` (`self.Current Id`)
        (:`0`
          _)
        (:`1`
          _)
        (:`2`
          _))
      (`self.OnEventComplete`))
    (:`then_1`
      (`/Engine/EditorBlueprintResources/StandardMacros.IsValid` _value
        (:`Is Valid`
          (`self.K2_DestroyActor` _value)
          (bind _result (`/Engine/EditorBlueprintResources/StandardMacros.IncrementInt` (`self.Current Id`))
            (:`  `
              (bind _value_2 (`BlueprintMapLibrary.Map_Find` (`self.Triggers`) _result))
              (`/Engine/EditorBlueprintResources/StandardMacros.IsValid` _value_2
                (:`Is Valid`
                  (set `/Game/Test_Horror/Blueprints/Item/BP_Collectible.Active` true _value_2))))))))))

(fn `UserConstructionScript`)